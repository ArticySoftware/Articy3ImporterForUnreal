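; BP_ArticyFlowDebugger is a debugging Blueprint that shows an on-screen widget for an Articy flow player.
; On BeginPlay it creates W_ArticyDebugger with a reference to itself, adds it to the viewport, then re-sets the FlowPlayer's start node to retrigger it.
; ShowDebugWidget toggles the widget by adding it to or removing it from the viewport.
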(event EventBeginPlay
  (bind _flowplayer (Variables|Default|GetFlowPlayer))
  (bind _returnvalue (UserInterface|CreateWidget "/ArticyImporter/UI/W_ArticyDebugger.W_ArticyDebugger_C" 0 self))
  (bind _output_get (Variables|Default|SetArticyDebugWidget _returnvalue))
  (UserInterface|Viewport|AddtoViewport _output_get 0)
  ;[1 1 1] Retrigger the same start node
  (Class|ArticyFlowPlayer|SetStartNode _flowplayer (Variables|/Script/ArticyRuntime.ArticyFlowPlayer|GetStartOn _flowplayer)))

(event EventTick
  (params (DeltaSeconds :type Float%20%28single-precision%29)))

(fn ConstructionScript)

(fn ShowDebugWidget
  (params (Show :type Boolean))
  (bind _articydebugwidget (Variables|Default|GetArticyDebugWidget))
  (if Show
    (UserInterface|Viewport|AddtoViewport _articydebugwidget 0)
    (else
      (Widget|RemovefromParent _articydebugwidget))))